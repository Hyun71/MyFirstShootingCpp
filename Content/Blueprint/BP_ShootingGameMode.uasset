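; Game mode for a shooting game that tracks the score and shows the game-over screen.
; AddScore adds a value to the running Score.
; ShowGameOverUIa creates the WBP_GameOver widget only if none is valid, then shows the cursor and switches to UI-only input.
; The event graph does nothing at runtime: its events are empty, and the nodes for score widget creation and game-only input are disconnected.
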(event EventBeginPlay)

(event EventTick
  (params (DeltaSeconds :type Float%20%28single-precision%29)))

(event EventInitializeHUDforPlayer
  (params (NewPlayer :type Player%20Controller%20Object%20Reference))
  ;[1 1 1] 초기화.
)

(fn ConstructionScript)

(fn AddScore
  (params (value :type Integer))
  (Variables|Default|SetScore (+ value (Variables|Default|GetScore))))

(fn ShowGameOverUIa
  (bind _returnvalue (Game|GetPlayerController 0))
  (Utilities|IsValid (Variables|Default|GetGameOverUI)
    (:Is%20Not%20Valid
      (bind _returnvalue_2 (UserInterface|CreateWidget "/Game/UI/WBP_GameOver.WBP_GameOver_C"))
      (bind _output_get (Variables|Default|SetGameOverUI _returnvalue_2))
      (UserInterface|Viewport|AddtoViewport _output_get 0)
      (Variables|/Script/Engine.PlayerController|SetbShowMouseCursor _returnvalue true)
      (Input|SetInputModeUIOnly _returnvalue 0 "DoNotLock"))))